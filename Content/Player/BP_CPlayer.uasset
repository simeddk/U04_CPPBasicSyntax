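; BP_CPlayer is a player Blueprint that handles camera zoom and holds a reference to a target point.
; Zoomin plays a timeline that drives the camera's field of view, and ZoomOut reverses it.
; BeginPlay stores the first BP_TargetPoint found in the level.
; An unconnected debug branch would print a spine pitch angle toward that target, but it never runs, and Tick is empty.
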(event `self.ReceiveBeginPlay`
  (bind _outactors (`GameplayStatics.GetAllActorsOfClass` "/Game/04_BoneTransform/BP_TargetPoint.BP_TargetPoint_C"))
  (set `self.TargetPoint` (`|GetArrayItem` _outactors)))

(event `self.ZoomIn`
  (bind (_direction _fov) (`Timeline|ZoomTimeline` :!label _label)
    (:`Update`
      (`CameraComponent.SetFieldOfView` (`self.Camera`) _fov))))

(event `self.ZoomOut`
  (goto _label :!via `Reverse`))

(event `self.ReceiveTick`
  (params (DeltaSeconds :type "Float (single-precision)")))

(fn `UserConstructionScript`)